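; Sphere actor that reacts to gaze and overlap exit, driving its own material and that of linked Objects.
; BeginPlay creates dynamic materials, with all Objects sharing one instance.
; StartGaze and StopGaze run a timeline on the sphere's "div" parameter, while exit reverses the Objects' opacity timeline and starts Amplitude-scaled vertical motion.
; Enter overlap is empty; its logic, light dimming, attachment and scaling are disconnected.
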(event OnComponentBeginOverlap(Sphere_enter)
  (params (OverlappedComponent :type Primitive%20Component%20Object%20Reference) (OtherActor :type Actor%20Object%20Reference) (OtherComp :type Primitive%20Component%20Object%20Reference) (OtherBodyIndex :type Integer) (bFromSweep :type Boolean) (SweepResult :type Hit%20Result%20Structure%20%28by%20ref%29)))

(event OnComponentEndOverlap(Sphere_exit)
  (params (OverlappedComponent :type Primitive%20Component%20Object%20Reference) (OtherActor :type Actor%20Object%20Reference) (OtherComp :type Primitive%20Component%20Object%20Reference) (OtherBodyIndex :type Integer))
  (Utilities|FlowControl|Sequence
    (:then_0
      (Development|PrintString "Exit")
      (Components|Timeline|SetPlayRate (Variables|Default|GetTimeline_0) 4.0)
      (bind _newtrack_0 (Timeline|Timeline_0 ReverseFromEnd)
        (:Update
          (for _array_element (Variables|Default|GetMats)
            (Rendering|Material|SetScalarParameterValue _array_element "OpacityLevel" _newtrack_0 :!class /Script/Engine.MaterialInstanceDynamic))
          (if (Variables|Default|GetSwitchOffLiht)
            _))))
    (:then_1
      (bind _newtrack_0_2 (Timeline|Timeline_2 Play)
        (:Update
          (Transformation|AddLocalOffset (Variables|Default|GetDefaultSceneRoot) (Math|Vector|MakeVector 0.0 0.0 (* (* _newtrack_0_2 0.2) (Variables|Default|GetAmplitude))) false false))))))

(event Custom|StartGaze
  (Development|PrintString "StartGaze")
  (bind _newtrack_0 (Timeline|Timeline_1 PlayFromStart)
    (:Update
      (Rendering|Material|SetScalarParameterValue (Variables|Default|GetMyMat) "div" _newtrack_0 :!class /Script/Engine.MaterialInstanceDynamic))))

(event Custom|StopGaze
  (Development|PrintString "StopGaze")
  (bind _newtrack_0 (Timeline|Timeline_1 ReverseFromEnd)
    (:Update
      (Rendering|Material|SetScalarParameterValue (Variables|Default|GetMyMat) "div" _newtrack_0 :!class /Script/Engine.MaterialInstanceDynamic))))

(event EventBeginPlay
  (bind _objects (Variables|Default|GetObjects))
  (bind _sphere (Variables|Default|GetSphere))
  (bind _mats (Variables|Default|GetMats))
  (Utilities|Array|Add (Variables|Default|GetIgnoreSpheres) (Variables|Default|GetPawn))
  (if (Variables|Default|GetSwitchOffLiht)
    (Variables|Default|SetStartLight (Variables|/Script/Engine.LightComponentBase|GetIntensity (Variables|/Script/Engine.Light|GetLightComponent (Variables|Default|GetLight)))))
  (for _array_element (Variables|Default|GetInnerIndex)
    _)
  (bind _returnvalue (Rendering|Material|CreateDynamicMaterialInstance (Rendering|Material|GetMaterial _sphere 0) "None" :!class /Script/Engine.KismetMaterialLibrary))
  (bind _output_get (Variables|Default|SetMyMat _returnvalue))
  (Rendering|Material|SetMaterial _sphere 0 _output_get)
  (if (> (Utilities|Array|Length _objects) 0)
    (bind _returnvalue_2 (Rendering|Material|CreateDynamicMaterialInstance (Rendering|Material|GetMaterial (Variables|/Script/Engine.StaticMeshActor|GetStaticMeshComponent (Utilities|Array|Get(acopy) _objects)) 0) "None" :!class /Script/Engine.KismetMaterialLibrary))
    (Utilities|Array|Add _mats _returnvalue_2)
    (for _array_element_2 _objects
      (Rendering|Material|SetMaterial (Variables|/Script/Engine.StaticMeshActor|GetStaticMeshComponent _array_element_2) 0 (Utilities|Array|Get(acopy) _mats))
      (Rendering|Material|SetScalarParameterValue (Variables|Default|GetMyMat) "div" 3.0 :!class /Script/Engine.MaterialInstanceDynamic))))

(fn ConstructionScript)