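; BP_Sphere is an actor that experiments with child actors and runtime spawning and attachment.
; When SpawnSphere is set, its construction script adds a BP_sec_child child actor component and attaches that actor to the root.
; Pressing 9 detaches the BPSecChild actor, clears its owner, then spawns another BP_Sphere attached to itself.
; A Delete event destroys that spawned sphere, but its construction script call is disconnected.
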(event Custom|Spawn
  (Development|PrintString "Spawn Sphere")
  (bind _returnvalue (AddComponent|AddChildActorComponent false))
  (ChildActorComponent|SetChildActorClass _returnvalue "/Game/MyContent/Blueprints/trash/BP_sec_child.BP_sec_child_C")
  (Transformation|AttachComponentToComponent (Variables|/Script/Engine.ChildActorComponent|GetChildActor _returnvalue) (Variables|Default|GetDefaultSceneRoot) "None" "KeepRelative" "KeepRelative" "KeepRelative" true))

(event Custom|Delete
  (Development|PrintString "Delete Sphere")
  (Actor|DestroyActor (stale Input|KeyboardEvents|9 _returnvalue)))

(event Input|KeyboardEvents|9
  (params (Key :type Key%20Structure))
  (bind _bp_sec_child (Variables|Default|GetBP_sec_child))
  (bind _childactor (Variables|/Script/Engine.ChildActorComponent|GetChildActor _bp_sec_child))
  (:Pressed
    (Transformation|DetachFromActor _childactor "KeepWorld" "KeepWorld" "KeepWorld")
    (Actor|SetOwner _childactor 0)
    (bind _returnvalue (Game|SpawnActorfromClass "BP_Sphere_C" (Math|Transform|MakeTransform "0, 0, 0" "0, 0, 0" "1,1,1") "AlwaysSpawn" 0 0))
    (Transformation|AttachActorToActor _returnvalue self "None" "KeepWorld" "KeepWorld" "KeepWorld" true)))

(fn ConstructionScript
  (if (Variables|Default|GetSpawnSphere)
    (CallFunction|Spawn)))