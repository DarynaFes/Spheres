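; Environment dune Blueprint that plays a one-shot hands animation on one of its skeletal meshes.
; On BeginPlay it waits a random delay of several seconds, then randomly picks one of three skeletal mesh components to play the same non-looping animation.
; The animation fires only once per instance, and the construction script only calls its parent.
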(event EventBeginPlay
  (|CallParentFunction)
  (Utilities|FlowControl|Delay (Math|Random|RandomFloatinRange 5.0 2e+01))
  (switch int (Math|Random|RandomIntegerinRange 0 2)
    (:0
      (Components|Animation|PlayAnimation (Variables|Default|GetSkeletalMesh) "/Game/MyContent/Animations/Just_some_Hands_Cube_000_Anim_Default_Take.Just_some_Hands_Cube_000_Anim_Default_Take" false))
    (:1
      (Components|Animation|PlayAnimation (Variables|Default|GetSkeletalMesh1) "/Game/MyContent/Animations/Just_some_Hands_Cube_000_Anim_Default_Take.Just_some_Hands_Cube_000_Anim_Default_Take" false))
    (:2
      (Components|Animation|PlayAnimation (Variables|Default|GetSkeletalMesh2) "/Game/MyContent/Animations/Just_some_Hands_Cube_000_Anim_Default_Take.Just_some_Hands_Cube_000_Anim_Default_Take" false))))

(fn ConstructionScript
  (|CallParentFunction))