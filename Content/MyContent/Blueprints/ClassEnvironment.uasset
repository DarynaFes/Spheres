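; Environment actor that, when DynMat is set, animates the opacity of its components' materials on BeginPlay.
; It swaps every material on the root's direct primitive children for a dynamic instance with OpacityLevel at zero, caching them in Mats.
; The slowed MatVisibility timeline then writes its track value to OpacityLevel on all cached instances each update.
; A three-second Delay leading into the timeline is left disconnected.
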(event EventBeginPlay
  (Development|PrintString "Environment created")
  (if (Variables|Default|GetDynMat)
    (for _array_element (Components|GetChildrenComponents (Variables|Default|GetDefaultSceneRoot) false)
      (bind _asprimitive_component (Utilities|Casting|CastToPrimitiveComponent _array_element))
      (for _index (range 0 (- (Rendering|Material|GetNumMaterials _asprimitive_component) 1))
        (bind _returnvalue (Rendering|Material|CreateDynamicMaterialInstance (Rendering|Material|GetMaterial _asprimitive_component _index) "None" :!class /Script/Engine.KismetMaterialLibrary))
        (Utilities|Array|Add (Variables|Default|GetMats) _returnvalue)
        (Rendering|Material|SetMaterial _asprimitive_component _index _returnvalue)
        (Rendering|Material|SetScalarParameterValue _returnvalue "OpacityLevel" 0.0 :!class /Script/Engine.MaterialInstanceDynamic)))
    (Components|Timeline|SetPlayRate (Variables|Default|GetMatVisibility) 0.4)
    (bind _newtrack_0 (Timeline|MatVisibility PlayFromStart)
      (:Update
        (for _array_element_2 (Variables|Default|GetMats)
          (Rendering|Material|SetScalarParameterValue _array_element_2 "OpacityLevel" _newtrack_0 :!class /Script/Engine.MaterialInstanceDynamic))))))

(fn ConstructionScript)