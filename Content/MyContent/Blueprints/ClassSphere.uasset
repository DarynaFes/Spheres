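; Gaze-selectable sphere actor that the player moves into, revealing an attached environment and nested inner spheres.
; Gazing plays reversible timelines driving a camera-facing loader and sphere lighting, then calls MoveToNewSphere on the pawn when finished.
; Entry overlap, or BeginPlay for start spheres, spawns contents, fades in audio and disables gaze; exit overlap notifies the pawn.
; Other spheres zoom in and bob from random phases; construction script optionally previews contents.
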(event OnComponentBeginOverlap(Sphere_enter)
  (params (OverlappedComponent :type Primitive%20Component%20Object%20Reference) (OtherActor :type Actor%20Object%20Reference) (OtherComp :type Primitive%20Component%20Object%20Reference) (OtherBodyIndex :type Integer) (bFromSweep :type Boolean) (SweepResult :type Hit%20Result%20Structure%20%28by%20ref%29))
  (if (not (Variables|Default|GetSpawn_on_Start))
    (Development|PrintString "Sphere Collision start")
    (Utilities|FlowControl|DoOnce false
      (:Completed
        (Development|PrintString "Sphere spawn 1" true true "(R=0.130269,G=1.000000,B=0.086891,A=1.000000)")
        (CallFunction|SpawnObjects)))))

(event OnComponentBeginOverlap(Sphere_exit)
  (params (OverlappedComponent :type Primitive%20Component%20Object%20Reference) (OtherActor :type Actor%20Object%20Reference) (OtherComp :type Primitive%20Component%20Object%20Reference) (OtherBodyIndex :type Integer) (bFromSweep :type Boolean) (SweepResult :type Hit%20Result%20Structure%20%28by%20ref%29))
  (Utilities|FlowControl|DoOnce false
    (:Completed
      (Default|SphereEntered (Variables|Default|GetMyPawn)))))

(event Custom|StartGaze
  ;[0 1 0.2311] Gaze -change color
  (Utilities|FlowControl|Gate false
    (:Exit
      (Development|PrintString "StartGaze")
      (Utilities|FlowControl|Sequence
        (:then_0
          (bind _newtrack_0 (Timeline|GazeTimer Play)
            (:Update
              (Development|PrintString (Utilities|String|ToString(Float) _newtrack_0))
              (Rendering|Material|SetScalarParameterValue (Variables|Default|GetLoaderMat) "Level1" _newtrack_0 :!class /Script/Engine.MaterialInstanceDynamic))
            (:Finished
              (Default|MovetoNewSphere (Variables|Default|GetMyPawn)))))
        (:then_1
          (bind _newtrack_0_2 (Timeline|GazeLightning Play)
            (:Update
              (Rendering|Material|SetScalarParameterValue (Variables|Default|GetMyMat) "div" (Math|Float|MapRangeClamped _newtrack_0_2 0.0 1.0 (Variables|Default|GetLight_Gazed) (Variables|Default|GetLight_NOT_Gazed)) :!class /Script/Engine.MaterialInstanceDynamic))))))))

(event Custom|StopGaze
  ;[0 1 0.2311] Gaze -change color
  (Utilities|FlowControl|Gate false
    (:Exit
      (Development|PrintString "StopGaze")
      (Utilities|FlowControl|Sequence
        (:then_0
          (bind _newtrack_0 (Timeline|GazeTimer Reverse)
            (:Update
              (Development|PrintString (Utilities|String|ToString(Float) _newtrack_0))
              (Rendering|Material|SetScalarParameterValue (Variables|Default|GetLoaderMat) "Level1" _newtrack_0 :!class /Script/Engine.MaterialInstanceDynamic))
            (:Finished
              (Default|MovetoNewSphere (Variables|Default|GetMyPawn)))))
        (:then_1
          (bind _newtrack_0_2 (Timeline|GazeLightning Reverse)
            (:Update
              (Rendering|Material|SetScalarParameterValue (Variables|Default|GetMyMat) "div" (Math|Float|MapRangeClamped _newtrack_0_2 0.0 1.0 (Variables|Default|GetLight_Gazed) (Variables|Default|GetLight_NOT_Gazed)) :!class /Script/Engine.MaterialInstanceDynamic))))))))

(event Custom|SpawnObjects
  (bind _environment (Variables|Default|GetEnvironment))
  ;[0.1261 0.05415 1] Spawn Objects
  (Development|PrintString "SPAWN" true true "(R=1.000000,G=0.000000,B=0.096778,A=1.000000)")
  (Actor|Tick|SetActorTickEnabled false)
  (Components|DestroyComponent (Variables|Default|GetWidget))
  (Collision|SetCollisionEnabled (Variables|Default|GetGazeCollision) "NoCollision")
  (Utilities|FlowControl|Sequence
    (:then_0
      (Utilities|FlowControl|DoOnce false
        (:Completed
          (Rendering|Material|SetScalarParameterValue (Variables|Default|GetMyMat) "div" (Variables|Default|GetLight_Gazed) :!class /Script/Engine.MaterialInstanceDynamic)
          (Utilities|FlowControl|Sequence
            (:then_0
              (if (Utilities|IsValidClass _environment)
                (bind _returnvalue (Game|SpawnActorfromClass _environment (Transformation|GetWorldTransform (Variables|Default|GetDefaultSceneRoot)) "AlwaysSpawn" 0 0))
                (Transformation|AttachActorToActor _returnvalue self "None" "KeepWorld" "KeepWorld" "KeepWorld" true)
                (else
                  (Development|PrintString "No Environment")))
              (for (_array_element _array_index) (Variables|Default|GetInnerSpheres)
                (bind _returnvalue_2 (Game|SpawnActorfromClass _array_element (Utilities|Array|Get(acopy) (Variables|Default|GetInnerSpheres_Transform) _array_index) "AlwaysSpawn" 0 0))
                (Transformation|AttachActorToActor _returnvalue_2 self "None" "KeepRelative" "KeepRelative" "KeepRelative" false)))
            (:then_1
              (bind _soundlevel (Timeline|SoundTimeline Play)
                (:Update
                  (Audio|Components|Audio|AdjustVolume (Variables|Default|GetSphere_audio) 0.0 (* _soundlevel (Variables|Default|GetSoundLevel)) :!class /Script/Engine.AudioComponent))))))))
    (:then_1
      ;[0 1 0.2311] Gaze -change color
      (Utilities|FlowControl|Sequence
        (:then_0
          (Utilities|FlowControl|Gate false) ; enters at Close
        )
        (:then_1
          (Utilities|FlowControl|Gate false) ; enters at Close
        )))))

(event Custom|DestroySphereAndObj
  ;[0.1261 0.05415 1] Spawn Objects
  (bind _output_get (Variables|Default|SetNumActors (Utilities|Array|Length (Actor|GetAttachedActors self))))
  (for _index (range 1 _output_get)
    (Actor|DestroyActor (Utilities|Array|Get(acopy) (Actor|GetAttachedActors self))))
  (Actor|DestroyActor))

(event Custom|StopMovement
  ;[1 0 0] Init at start
  (bind _newtrack_0 (Timeline|SphereMovementTimeline Stop)
    (:Update
      (Transformation|AddLocalOffset (Variables|Default|GetDefaultSceneRoot) (Math|Vector|MakeVector 0.0 0.0 (* (Math|Float|Sign(Float) _newtrack_0) (Variables|Default|GetDelta))) false false))))

(event EventBeginPlay
  (bind _widget (Variables|Default|GetWidget))
  ;[1 0 0] Init at start
  (Variables|Default|Setis_main (Variables|Default|GetSpawn_on_Start))
  (bind _aswidget_timer (Utilities|Casting|CastToWidget_Timer (UserInterface|GetUserWidgetObject (Variables|Default|GetWidget))))
  (Appearance|SetColorandOpacity _aswidget_timer (Math|Conversions|ToLinearColor(Color) (Variables|Default|GetLoaderColor)) :!class /Script/UMG.UserWidget)
  (bind _returnvalue (Rendering|Material|CreateDynamicMaterialInstance (Variables|Default|GetWidget) 0 (Rendering|Material|GetMaterial _widget 0) "None" :!class /Script/Engine.PrimitiveComponent))
  (bind _output_get (Variables|Default|SetLoaderMat _returnvalue))
  (Rendering|Material|SetMaterial _widget 0 _output_get)
  (bind _asmy_pawn (Utilities|Casting|CastToMyPawn (Game|Player|GetPlayerPawn 0)))
  (Variables|Default|SetMyPawn _asmy_pawn)
  (Audio|Components|Audio|AdjustVolume (Variables|Default|GetSphere_audio) 0.0 0.0 :!class /Script/Engine.AudioComponent)
  (Development|PrintString "SphereCreated")
  (Components|Timeline|SetPlayRate (Variables|Default|GetSphereMovementTimeline) 0.5)
  (Variables|Default|SetStartTime (Math|Random|RandomFloatinRange 0.0 8.0))
  (bind _returnvalue_2 (Rendering|Material|CreateDynamicMaterialInstance (Rendering|Material|GetMaterial (Variables|Default|GetSphere) 0) "None" :!class /Script/Engine.KismetMaterialLibrary))
  (bind _output_get_2 (Variables|Default|SetMyMat _returnvalue_2))
  (Rendering|Material|SetMaterial (Variables|Default|GetSphere) 0 _output_get_2)
  (Rendering|Material|SetScalarParameterValue (Variables|Default|GetMyMat) "div" (Variables|Default|GetLight_NOT_Gazed) :!class /Script/Engine.MaterialInstanceDynamic)
  (if (Variables|Default|GetSpawn_on_Start)
    (CallFunction|SpawnObjects)
    (Variables|/Script/Engine.PrimitiveComponent|SetbGenerateOverlapEvents (Variables|Default|GetSphere_exit) false)
    (Variables|/Script/Engine.PrimitiveComponent|SetbGenerateOverlapEvents (Variables|Default|GetSphere_enter) true)
    (else
      (Utilities|FlowControl|Sequence
        (:then_0
          (Components|Timeline|SetPlaybackPosition (Variables|Default|GetSphereMovementTimeline) (Variables|Default|GetStartTime) false false)
          (bind _newtrack_0 (Timeline|SphereMovementTimeline Play)
            (:Update
              (Transformation|AddLocalOffset (Variables|Default|GetDefaultSceneRoot) (Math|Vector|MakeVector 0.0 0.0 (* (Math|Float|Sign(Float) _newtrack_0) (Variables|Default|GetDelta))) false false))))
        (:then_2
          (Variables|Default|SetStartSize (.x (Variables|/Script/Engine.SceneComponent|GetRelativeScale3D (Variables|Default|GetDefaultSceneRoot))))
          (bind _newtrack_0_2 (Timeline|ZoomIn Play)
            (:Update
              (Transformation|SetRelativeScale3D (Variables|Default|GetDefaultSceneRoot) (Math|Vector|MakeVector (* (Variables|Default|GetStartSize) _newtrack_0_2) (* (Variables|Default|GetStartSize) _newtrack_0_2) (* (Variables|Default|GetStartSize) _newtrack_0_2))))
            (:Finished
              (Variables|/Script/Engine.PrimitiveComponent|SetbGenerateOverlapEvents (Variables|Default|GetSphere_exit) true)
              (Variables|/Script/Engine.PrimitiveComponent|SetbGenerateOverlapEvents (Variables|Default|GetSphere_enter) true))))))))

(event EventTick
  (params (DeltaSeconds :type Float%20%28single-precision%29))
  (Transformation|SetWorldRotation (Variables|Default|GetWidget) (Math|Rotator|FindLookatRotation (Transformation|GetWorldLocation (Variables|Default|GetWidget)) (Transformation|GetWorldLocation (Variables|/Game/MyContent/Blueprints/MyPawn.MyPawn_C|GetCamera (Variables|Default|GetMyPawn)))) false false))

(event Input|KeyboardEvents|SpaceBar
  (params (Key :type Key%20Structure))
  ;[1 1 1] Debug
  (:Pressed
    (CallFunction|SpawnObjects)))

(event Input|KeyboardEvents|Enter
  (params (Key :type Key%20Structure))
  ;[1 1 1] Debug
  (:Pressed
    (CallFunction|DestroySphereandObj)))

(fn ConstructionScript
  (if (Variables|Default|GetSpawnObj_DEBUG)
    (bind _returnvalue (AddComponent|AddChildActorComponent false))
    (if (Utilities|IsValidClass (Variables|Default|GetEnvironment))
      (ChildActorComponent|SetChildActorClass _returnvalue (Variables|Default|GetEnvironment))
      (Transformation|AttachComponentToComponent (Variables|/Script/Engine.ChildActorComponent|GetChildActor _returnvalue) (Variables|Default|GetDefaultSceneRoot) "None" "KeepWorld" "KeepWorld" "KeepWorld" true))
    (for (_array_element _array_index) (Variables|Default|GetInnerSpheres)
      (bind _returnvalue_2 (AddComponent|AddChildActorComponent false (Utilities|Array|Get(acopy) (Variables|Default|GetInnerSpheres_Transform) _array_index)))
      (ChildActorComponent|SetChildActorClass _returnvalue_2 _array_element)
      (Transformation|AttachComponentToComponent (Variables|/Script/Engine.ChildActorComponent|GetChildActor _returnvalue_2) (Variables|Default|GetDefaultSceneRoot) "None" "KeepWorld" "KeepWorld" "KeepWorld" false))))