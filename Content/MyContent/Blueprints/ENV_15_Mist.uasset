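; ENV_15_Mist is an environment actor that animates a static mesh growing in and continuously rotating.
; On BeginPlay, the SizeCube timeline drives a uniform scale-up of the mesh from zero to slightly under full size.
; Tick constantly tumbles the mesh in roll and pitch, and a gate opened when the timeline finishes adds a slow yaw to the Scene component.
; Both rotations use fixed per-frame increments, so their speed depends on frame rate.
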(event EventBeginPlay
  (|CallParentFunction)
  (bind _newtrack_0 (Timeline|SizeCube PlayFromStart)
    (:Update
      (Transformation|SetRelativeScale3D (Variables|Default|GetStaticMesh) (Math|Vector|MakeVector (Math|Float|MapRangeClamped _newtrack_0 0.0 1.0 0.0 0.9) (Math|Float|MapRangeClamped _newtrack_0 0.0 1.0 0.0 0.9) (Math|Float|MapRangeClamped _newtrack_0 0.0 1.0 0.0 0.9))))
    (:Finished
      (Utilities|FlowControl|Gate true) ; enters at Open
    )))

(event Collision|EventActorBeginOverlap
  (params (OtherActor :type Actor%20Object%20Reference)))

(event EventTick
  (params (DeltaSeconds :type Float%20%28single-precision%29))
  (Transformation|AddLocalRotation (Variables|Default|GetStaticMesh) (Math|Rotator|MakeRotator 0.04 0.025 0.0) false false)
  (Utilities|FlowControl|Gate true
    (:Exit
      (Transformation|AddLocalRotation (Variables|Default|GetScene) "0,0.015000, 0" false false))))

(fn ConstructionScript
  (|CallParentFunction))